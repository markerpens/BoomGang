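; Lobby player controller that puts each player on the lobby camera and shows team selection.
; On BeginPlay the server possesses the first LobbyView actor, while the local controller opens the TeamSelection widget with UI-only input and a visible cursor.
; The TeamSelected event passes the chosen team and this controller to LobbyGameMode's RequestSpawn, intended to run server-side.
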(event `self.ReceiveBeginPlay`
  (bind _returnvalue (`GameplayStatics.GetPlayerController` 0))
  (`|ExecutionSequence`
    (:`then_0`
      ;[1 1 1] Possess lobby camera on server
      (`/Engine/EditorBlueprintResources/ActorMacros.Switch Has Authority`
        (:`Authority`
          (bind _outactors (`GameplayStatics.GetAllActorsOfClass` "/Game/LobbyBP/Blueprints/LobbyView.LobbyView_C"))
          (`self.Possess` (`|GetArrayItem` _outactors)))))
    (:`then_1`
      ;[1 1 1] Create widget on local
      (if (`self.IsLocalController`)
        (bind _returnvalue_2 (`|CreateWidget` "/Game/LobbyBP/Blueprints/Widgets/TeamSelection.TeamSelection_C"))
        (`UserWidget.AddToViewport` _returnvalue_2 0)
        (`WidgetBlueprintLibrary.SetInputMode_UIOnlyEx` _returnvalue null)
        (set `PlayerController.bShowMouseCursor` true _returnvalue)))))

(event `TeamSelected`
  (params (`Team Selected` :type "/Game/LobbyBP/Blueprints/Teams Enum" :default "NewEnumerator0"))
  ;[1 1 1] Select team on server-side
  (`/Game/LobbyBP/Blueprints/LobbyGameMode.RequestSpawn` (cast `/Game/LobbyBP/Blueprints/LobbyGameMode` (`GameplayStatics.GetGameMode`) :!pure true) `Team Selected` self))

(fn `UserConstructionScript`)